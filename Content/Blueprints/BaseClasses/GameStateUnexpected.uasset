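; Game state base class that provides helper functions for showing dialog boxes and two-button questions to the player.
; CreateDialogBox disables player character input, shows the mouse cursor, then displays a DialogBox widget and starts its text scrolling with the given delay.
; For questions, CreateChoiceBox builds a DialogChoice widget from two button structs, which is handed to the dialog box without being added to the viewport here.
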(event EventBeginPlay)

(fn ConstructionScript)

(fn CreateDialogBox
  (params (Dialog%20Text :type Text) (TextDelay :type Float%20%28single-precision%29) (isQuestion :type Boolean) (Button1 :type Button%20Structure) (Button2 :type Button%20Structure))
  (bind _returnvalue (UserInterface|CreateWidget "/Game/Blueprints/BaseClasses/DialogBox.DialogBox_C")) ; Spawn an instance
  (LocalVariables|SetDialogWidget _returnvalue)
  (Input|DisableInput (Game|GetPlayerCharacter 0) 0)
  (Variables|/Script/Engine.PlayerController|SetbShowMouseCursor (Game|GetPlayerController 0) true)
  (Variables|/Game/Blueprints/BaseClasses/DialogBox.DialogBox_C|SetDialogText (LocalVariables|GetDialogWidget) Dialog%20Text)
  (Variables|/Game/Blueprints/BaseClasses/DialogBox.DialogBox_C|SetTextDelay (LocalVariables|GetDialogWidget) TextDelay)
  (if isQuestion
    ;[1 1 1] Create a choice box to display after the dialog box
    (Variables|/Game/Blueprints/BaseClasses/DialogBox.DialogBox_C|SetisQuestion (LocalVariables|GetDialogWidget) true)
    (bind _choiceboxresult (CallFunction|CreateChoiceBox Button1 Button2))
    (Variables|/Game/Blueprints/BaseClasses/DialogBox.DialogBox_C|SetChoiceBox (LocalVariables|GetDialogWidget) _choiceboxresult))
  ;[1 1 1] Show the dialog box
  (UserInterface|Viewport|AddtoViewport (LocalVariables|GetDialogWidget) 0)
  (Default|StartScrolling (LocalVariables|GetDialogWidget)))

(fn CreateChoiceBox
  (params (Button1 :type Button%20Structure) (Button2 :type Button%20Structure))
  (bind _returnvalue (UserInterface|CreateWidget "/Game/Blueprints/BaseClasses/DialogChoice.DialogChoice_C"))
  (bind _output_get (LocalVariables|SetDialogWidget _returnvalue))
  (Variables|/Game/Blueprints/BaseClasses/DialogChoice.DialogChoice_C|SetButton1Struct _output_get Button1)
  (Variables|/Game/Blueprints/BaseClasses/DialogChoice.DialogChoice_C|SetButton2Struct _output_get Button2)
  (return _output_get))