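; DialogTriggerBase is a trigger Blueprint that opens a dialog box when its Trigger event fires.
; Trigger passes the dialog text, question flag and two button text/response pairs to WorldState's CreateDialogBox, then switches the player to UI-only input.
; The overlap events are empty, leaving their old input-toggle and FirstPersonCharacter interact-prompt logic disconnected and unused.
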(event Collision|EventActorBeginOverlap
  (params (OtherActor :type Actor%20Object%20Reference))
  ;[1 1 1] OLD Delete
)

(event Collision|EventActorEndOverlap
  (params (OtherActor :type Actor%20Object%20Reference))
  ;[1 1 1] OLD Delete
)

(event EventTrigger
  (Default|CreateDialogBox (Variables|Default|GetWorldState) (Variables|Default|GetDialog) 0.05 (Variables|Default|GetisQuestion) (Utilities|Struct|MakeButton (Variables|Default|GetButton1%20Text) (Variables|Default|GetButton1%20Response)) (Utilities|Struct|MakeButton (Variables|Default|GetButton2%20Text) (Variables|Default|GetButton2%20Response)))
  (Input|SetInputModeUIOnly (Game|GetPlayerController 0) 0 "DoNotLock"))

(event Input|ActionEvents|InputActionInteract
  (params (Key :type Key%20Structure))
  ;[1 1 1] OLD Delete
)

(fn ConstructionScript
  (|CallParentFunction))